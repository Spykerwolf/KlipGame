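; Key pickup actor that spins in the level and disappears when touched.
; Tick adds a fixed yaw step to the Key component each frame, so spin speed depends on frame rate.
; Any overlap with the Box destroys the actor and plays a 2D pickup sound, without filtering the overlapping actor or recording the pickup.
; An unconnected node that would raise the key never runs.
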(event OnComponentBeginOverlap(Box)
  (params (OverlappedComponent :type Primitive%20Component%20Object%20Reference) (OtherActor :type Actor%20Object%20Reference) (OtherComp :type Primitive%20Component%20Object%20Reference) (OtherBodyIndex :type Integer) (bFromSweep :type Boolean) (SweepResult :type Hit%20Result%20Structure%20%28by%20ref%29))
  (Actor|DestroyActor)
  (Audio|PlaySound2D "/Game/Klip/Audio/key_pickup.key_pickup" 1.0 1.0 0.0 0 0))

(event EventTick
  (params (DeltaSeconds :type Float%20%28single-precision%29))
  (bind _key (Variables|Default|GetKey))
  (bind _relativerotation (Variables|/Script/Engine.SceneComponent|GetRelativeRotation _key))
  ;[1 1 1] Rotate Key
  (Transformation|SetRelativeRotation _key (Math|Rotator|MakeRotator (.roll _relativerotation) (.pitch _relativerotation) (+ (.yaw _relativerotation) 1.5)) false false))

(fn ConstructionScript)