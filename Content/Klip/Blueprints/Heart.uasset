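; Heart pickup that restores health to the player character on contact.
; It spins every tick and plays a timeline that bobs it with local offsets.
; Overlapping its sphere destroys it, sends the player negative damage as healing, plays a pickup sound and has the game mode's HUD refresh health.
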(event OnComponentBeginOverlap(Sphere)
  (params (OverlappedComponent :type Primitive%20Component%20Object%20Reference) (OtherActor :type Actor%20Object%20Reference) (OtherComp :type Primitive%20Component%20Object%20Reference) (OtherBodyIndex :type Integer) (bFromSweep :type Boolean) (SweepResult :type Hit%20Result%20Structure%20%28by%20ref%29))
  (bind _asplayer_character (Utilities|Casting|CastToPlayerCharacter OtherActor))
  (Actor|DestroyActor)
  (Class|BPIDamageable|TakeDamage(Message) _asplayer_character -1.0)
  (Audio|PlaySound2D "/Engine/VREditor/Sounds/UI/Object_PickUp.Object_PickUp" 1.0 1.0 0.0 0 0)
  (bind _asklip_game_mode (Utilities|Casting|CastToKlipGameMode (Game|GetGameMode)))
  (Default|UpdateHealth (Variables|/Game/Klip/Blueprints/KlipGameMode.KlipGameMode_C|GetHUD _asklip_game_mode)))

(event EventTick
  (params (DeltaSeconds :type Float%20%28single-precision%29))
  ;[1 1 1] Auto heart spin
  (Transformation|AddActorLocalRotation "0,5.000000, 0" false false)
  (bind _movement_key (Timeline|HeartSpin Play)
    (:Update
      (Transformation|AddActorLocalOffset _movement_key false false))))

(fn ConstructionScript)