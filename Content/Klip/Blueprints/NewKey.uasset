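; NewKey is a key pickup actor that spins every tick and moves by offsets from the KeySpin timeline.
; Any overlap on its capsule destroys it, with no check on the overlapping actor.
; It then sets the player character's key count to one rather than incrementing, prints a message, plays a pickup sound and refreshes the skull and key HUD through KlipGameMode.
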(event OnComponentBeginOverlap(Capsule)
  (params (OverlappedComponent :type Primitive%20Component%20Object%20Reference) (OtherActor :type Actor%20Object%20Reference) (OtherComp :type Primitive%20Component%20Object%20Reference) (OtherBodyIndex :type Integer) (bFromSweep :type Boolean) (SweepResult :type Hit%20Result%20Structure%20%28by%20ref%29))
  (Actor|DestroyActor)
  (bind _asplayer_character (Utilities|Casting|CastToPlayerCharacter (Game|GetPlayerCharacter 0)))
  (Variables|/Game/Klip/Blueprints/PlayerCharacter.PlayerCharacter_C|SetNumberOfKeys _asplayer_character 1)
  (Development|PrintString "Key acquired!!!")
  (Audio|PlaySound2D "/Game/Klip/Audio/key_pickup.key_pickup" 1.0 1.0 0.0 0 0)
  (Variables|Default|SetKeyDestroyed true)
  (bind _asklip_game_mode (Utilities|Casting|CastToKlipGameMode (Game|GetGameMode)))
  (Default|UpdateSkulls (Variables|/Game/Klip/Blueprints/KlipGameMode.KlipGameMode_C|GetHUD _asklip_game_mode))
  (Default|UpdateKey (Variables|/Game/Klip/Blueprints/KlipGameMode.KlipGameMode_C|GetHUD _asklip_game_mode)))

(event EventTick
  (params (DeltaSeconds :type Float%20%28single-precision%29))
  (if (not (Variables|Default|GetKeyDestroyed))
    (Transformation|AddActorLocalRotation "0,2.500000, 0" false false)
    (bind _movement_key (Timeline|KeySpin Play)
      (:Update
        (Transformation|AddActorLocalOffset _movement_key false false)))))

(fn ConstructionScript)