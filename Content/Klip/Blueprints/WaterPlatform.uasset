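; Water platform trap that reacts when the player character enters its trigger volume.
; On overlap it turns the platform red through a dynamic material instance, plays an alert sound and runs a timeline driving the platform's relative Z.
; Leaving the trigger only restores the grayish color; the reverse timeline is never run, so nothing here moves the platform back.
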(event OnComponentBeginOverlap(TriggerVolume)
  (params (OverlappedComponent :type Primitive%20Component%20Object%20Reference) (OtherActor :type Actor%20Object%20Reference) (OtherComp :type Primitive%20Component%20Object%20Reference) (OtherBodyIndex :type Integer) (bFromSweep :type Boolean) (SweepResult :type Hit%20Result%20Structure%20%28by%20ref%29))
  (if (== OtherActor (Game|GetPlayerCharacter 0))
    (Rendering|Material|SetVectorParameterValue (Variables|Default|GetDynamicMat) "Color" "(R=1.000000,G=0.000000,B=0.000000,A=1.000000)" :!class /Script/Engine.MaterialInstanceDynamic)
    (Audio|PlaySound2D "/Game/Klip/Audio/alert.alert" 1.0 1.0 0.0 0 0)
    (bind _waterplatform (Timeline|WaterPlatformTrap Play)
      (:Update
        (Transformation|SetRelativeLocation (Variables|Default|GetWaterPlatform) (Math|Vector|MakeVector 0.0 0.0 _waterplatform) false false)))))

(event OnComponentEndOverlap(TriggerVolume)
  (params (OverlappedComponent :type Primitive%20Component%20Object%20Reference) (OtherActor :type Actor%20Object%20Reference) (OtherComp :type Primitive%20Component%20Object%20Reference) (OtherBodyIndex :type Integer))
  (if (== OtherActor (Game|GetPlayerCharacter 0))
    (Rendering|Material|SetVectorParameterValue (Variables|Default|GetDynamicMat) "Color" "(R=0.545724,G=0.496933,B=0.520996,A=1.000000)" :!class /Script/Engine.MaterialInstanceDynamic)))

(event EventBeginPlay
  (bind _returnvalue (Rendering|Material|CreateDynamicMaterialInstance "/Game/Klip/Textures/PlatformChangeColor_Master.PlatformChangeColor_Master" "None" :!class /Script/Engine.KismetMaterialLibrary))
  (Variables|Default|SetDynamicMat _returnvalue)
  (Rendering|Material|SetMaterial (Variables|Default|GetWaterPlatform) 0 (Variables|Default|GetDynamicMat)))

(fn ConstructionScript)